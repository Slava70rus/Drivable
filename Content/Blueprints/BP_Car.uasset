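; Drivable car pawn with throttle, steering, handbrake, orbit camera, first/third-person switch, toggleable info widget and interface-based interaction with overlapping actors.
; FlipFlop inputs toggle headlights and play or reverse timelines that set door and wiper angle variables.
; Construction creates dynamic light materials, which brighten for headlights (alongside spotlights) and for brake lights on handbrake.
; Tick stores the larger-magnitude steer angle of the first two wheels as SteeringAngle.
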(event EventTick
  (params (DeltaSeconds :type Float%20%28single-precision%29))
  (CallFunction|SteeringWheelUpdate))

(event EventBeginPlay
  ;[1 1 1] UI
  (bind _returnvalue (UserInterface|CreateWidget "/Game/Blueprints/WBP_Information.WBP_Information_C"))
  (bind _output_get (Variables|Default|SetUI _returnvalue))
  (UserInterface|Viewport|AddtoViewport _output_get 0))

(event Input|ActionEvents|InputActionHandbrake
  (params (Key :type Key%20Structure :default "None"))
  (bind _back_light (Variables|Default|GetBack%20light))
  (bind _vehiclemovement (Variables|Default|GetVehicleMovement))
  ;[1 1 1] Handbrake
  (:Pressed
    (Class|WheeledVehicleMovementComponent|SetHandbrakeInput _vehiclemovement true)
    (Rendering|Material|SetScalarParameterValue _back_light "Light" 2e+02 :!class /Script/Engine.MaterialInstanceDynamic))
  (:Released
    (Class|WheeledVehicleMovementComponent|SetHandbrakeInput _vehiclemovement false)
    (Rendering|Material|SetScalarParameterValue _back_light "Light" 1.0 :!class /Script/Engine.MaterialInstanceDynamic)))

(event Input|ActionEvents|InputActionLightTrigger
  (params (Key :type Key%20Structure :default "None"))
  (bind _front_light (Variables|Default|GetFront%20light))
  ;[1 1 1] Lights
  (:Pressed
    (Utilities|FlowControl|FlipFlop
      (:A
        (Rendering|Material|SetScalarParameterValue _front_light "Light" 2e+02 :!class /Script/Engine.MaterialInstanceDynamic)
        (Rendering|SetVisibility (Variables|Default|GetRight%20SpotLight) true false)
        (Rendering|SetVisibility (Variables|Default|GetLeft%20SpotLightTop) true false)
        (Variables|Default|SetLights%20On true))
      (:B
        (Rendering|Material|SetScalarParameterValue _front_light "Light" 1.0 :!class /Script/Engine.MaterialInstanceDynamic)
        (Rendering|SetVisibility (Variables|Default|GetLeft%20SpotLight) false false)
        (Rendering|SetVisibility (Variables|Default|GetLeft%20SpotLightTop) false false)
        (Variables|Default|SetLights%20On false)))))

(event Input|ActionEvents|InputActionRightdoortrigger
  (params (Key :type Key%20Structure :default "None"))
  ;[1 1 1] Door functionality
  (:Pressed
    (Utilities|FlowControl|FlipFlop
      (:A
        (bind _door_anfle (Timeline|Right%20door Play)
          (:Update
            (Variables|Default|SetRight%20Door%20Angle _door_anfle))))
      (:B
        (Timeline|Right%20door Reverse)))))

(event Input|ActionEvents|InputActionWipers
  (params (Key :type Key%20Structure :default "None"))
  (:Pressed
    (if (Variables|Default|GetWipersCan)
      (Utilities|FlowControl|FlipFlop
        (:A
          (bind _door_anfle (Timeline|Timeline_0 Play)
            (:Update
              (Variables|Default|SetWipers%20Angle _door_anfle)
              (Variables|Default|SetWipersCan false))
            (:Finished
              (Variables|Default|SetWipersCan true))))
        (:B
          (Timeline|Timeline_0 Reverse))))))

(event Input|ActionEvents|InputActionInteract
  (params (Key :type Key%20Structure :default "None"))
  (:Pressed
    (bind _array_element (Utilities|Array|ForEachLoopwithBreak (Collision|GetOverlappingActors "/Script/Engine.Actor" :!class /Script/Engine.Actor) :!label _label)
      (:LoopBody
        (if (Utilities|DoesObjectImplementInterface _array_element "/Game/Blueprints/IBP_Interact.IBP_Interact_C")
          (Class|IBPInteract|Interact(Message) _array_element self)
          (goto _label Break))))))

(event Input|ActionEvents|InputActionLeftdoortrigger
  (params (Key :type Key%20Structure :default "None"))
  ;[1 1 1] Door functionality
  (:Pressed
    (Utilities|FlowControl|FlipFlop
      (:A
        (bind _door_anfle (Timeline|Left%20door Play)
          (:Update
            (Variables|Default|SetLeft%20Door%20Angle _door_anfle))))
      (:B
        (Timeline|Left%20door Reverse)))))

(event Input|ActionEvents|InputActionSwitchCamera
  (params (Key :type Key%20Structure :default "None"))
  (bind _1rd_person_camera (Variables|Default|Get1rd%20Person%20Camera))
  ;[1 1 1] Camera Switch
  (:Pressed
    (Utilities|FlowControl|FlipFlop
      (:A
        (Components|Activation|Deactivate (Variables|Default|Get3rd%20Person%20Camera))
        (Components|Activation|SetActive _1rd_person_camera true false)
        (Transformation|SetRelativeRotation _1rd_person_camera "-10.000000, 0, 0" false false))
      (:B
        (Components|Activation|Deactivate (Variables|Default|Get1rd%20Person%20Camera))
        (Components|Activation|SetActive (Variables|Default|Get3rd%20Person%20Camera) true false)
        (Transformation|SetRelativeRotation (Variables|Default|GetSpringArm) "-10.000000, 0, 0" false false)))))

(event Input|ActionEvents|InputActionUI
  (params (Key :type Key%20Structure :default "None"))
  (bind _ui (Variables|Default|GetUI))
  ;[1 1 1] UI
  (:Pressed
    (Utilities|FlowControl|FlipFlop
      (:A
        (Widget|RemovefromParent _ui))
      (:B
        (UserInterface|Viewport|AddtoViewport _ui 0)))))

(event Input|AxisEvents|InputAxisLookUp
  (params (AxisValue :type Float%20%28single-precision%29))
  (Transformation|AddRelativeRotation (Variables|Default|GetSpringArm) (Math|Rotator|MakeRotator 0.0 AxisValue 0.0) false false))

(event Input|AxisEvents|InputAxisLookRight
  (params (AxisValue :type Float%20%28single-precision%29))
  (Transformation|AddRelativeRotation (Variables|Default|GetSpringArm) (Math|Rotator|MakeRotator 0.0 0.0 AxisValue) false false))

(event Input|AxisEvents|InputAxisMoveForward
  (params (AxisValue :type Float%20%28single-precision%29))
  ;[1 1 1] Throttle and Steering
  (Class|WheeledVehicleMovementComponent|SetThrottleInput (Variables|Default|GetVehicleMovement) AxisValue))

(event Input|AxisEvents|InputAxisMoveRight
  (params (AxisValue :type Float%20%28single-precision%29))
  ;[1 1 1] Throttle and Steering
  (Class|WheeledVehicleMovementComponent|SetSteeringInput (Variables|Default|GetVehicleMovement) AxisValue))

(fn ConstructionScript
  (bind _mesh (Variables|Character|GetMesh))
  (bind _returnvalue (Rendering|Material|CreateDynamicMaterialInstance _mesh 8 "/Game/Material/M_front.M_front" "None" :!class /Script/Engine.PrimitiveComponent))
  (Variables|Default|SetFront%20light _returnvalue)
  (bind _returnvalue_2 (Rendering|Material|CreateDynamicMaterialInstance _mesh 12 "/Game/Material/M_back.M_back" "None" :!class /Script/Engine.PrimitiveComponent))
  (Variables|Default|SetBack%20light _returnvalue_2))

(fn SteeringWheelUpdate
  (bind _vehiclemovement (Variables|Default|GetVehicleMovement))
  (bind _wheels (Variables|/Script/PhysXVehicles.WheeledVehicleMovementComponent|GetWheels _vehiclemovement))
  (bind _output (Utilities|Array|Get(acopy) _wheels))
  (bind _output_2 (Utilities|Array|Get(acopy) _wheels 1))
  (bind _returnvalue (Class|VehicleWheel|GetSteerAngle _output_2))
  (bind _returnvalue_2 (Class|VehicleWheel|GetSteerAngle _output))
  (Variables|Default|SetSteering%20Angle (Math|Float|SelectFloat _returnvalue_2 _returnvalue (> (Math|Float|Absolute(Float) _returnvalue_2) (Math|Float|Absolute(Float) _returnvalue)))))