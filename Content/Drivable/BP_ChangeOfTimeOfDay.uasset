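; BP_ChangeOfTimeOfDay is a trigger that toggles the level between dimmed and full lighting when a BP_Car enters its box.
; Each overlap pitches, yaws or rolls nothing but the sun, turning the sky sphere's directional light half a turn in yaw.
; A FlipFlop alternates directional and sky light intensity, then the sky sphere updates its sun direction.
; Its text render spins continuously on Tick.
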(event OnComponentBeginOverlap(Box)
  (params (OverlappedComponent :type Primitive%20Component%20Object%20Reference) (OtherActor :type Actor%20Object%20Reference) (OtherComp :type Primitive%20Component%20Object%20Reference) (OtherBodyIndex :type Integer) (bFromSweep :type Boolean) (SweepResult :type Hit%20Result%20Structure%20%28by%20ref%29))
  (bind _skysphere (Variables|Default|GetSkySphere))
  (bind _skyl (Variables|Default|GetSkyL))
  (bind _directional_light_actor (Variables|/Engine/EngineSky/BP_Sky_Sphere.BP_Sky_Sphere_C|GetDirectional%20light%20actor _skysphere))
  (bind _lightcomponent (Variables|/Script/Engine.SkyLight|GetLightComponent _skyl))
  (bind _lightcomponent_2 (Variables|/Script/Engine.Light|GetLightComponent _directional_light_actor))
  (if (== (Utilities|GetClass OtherActor) "/Game/Drivable/BP_Car.BP_Car_C")
    (Transformation|AddLocalRotation (Variables|/Script/Engine.Actor|GetRootComponent _directional_light_actor) "180.000000, 0, 0" false false)
    (Utilities|FlowControl|FlipFlop
      (:A
        (Rendering|Components|Light|SetIntensity _lightcomponent_2 0.25)
        (Rendering|Components|Light|SetIntensity _lightcomponent 0.25))
      (:B
        (Rendering|Components|Light|SetIntensity _lightcomponent_2 1.0)
        (Rendering|Components|Light|SetIntensity _lightcomponent 1.0)))
    (Default|UpdateSunDirection _skysphere)))

(event EventTick
  (params (DeltaSeconds :type Float%20%28single-precision%29))
  (Transformation|AddLocalRotation (Variables|Default|GetTextRender) "0.000000,1.000000, 0" false false))

(fn ConstructionScript)